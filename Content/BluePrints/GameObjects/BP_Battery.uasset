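; BP_Battery is a pickup that recharges the first-person character's battery.
; When the player character overlaps its capsule collider, it adds a fixed amount to BatteryPower and caps it at a hardcoded limit rather than the character's BatteryPowerMAX.
; It then prints the new power value for debugging and destroys itself.
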(event `self.CapsuleCollider.OnComponentBeginOverlap`
  (params (OverlappedComponent :type "PrimitiveComponent Object Reference") (OtherActor :type "Actor Object Reference") (OtherComp :type "PrimitiveComponent Object Reference") (OtherBodyIndex :type Integer) (bFromSweep :type Boolean) (SweepResult :type "HitResult Structure (by ref)"))
  ;[1 1 1] Treat As
  (bind _asbp_first_person_character (cast `/Game/FirstPerson/Blueprints/BP_FirstPersonCharacter` OtherActor))
  (bind _battery_power_ (`/Game/FirstPerson/Blueprints/BP_FirstPersonCharacter.Battery Power ` _asbp_first_person_character))
  (bind _output_get (set `/Game/FirstPerson/Blueprints/BP_FirstPersonCharacter.Battery Power ` (+ _battery_power_ 25) _asbp_first_person_character))
  (if (> _output_get 100)
    (set `/Game/FirstPerson/Blueprints/BP_FirstPersonCharacter.Battery Power ` 100 _asbp_first_person_character)
    (`KismetSystemLibrary.PrintString` (`KismetStringLibrary.Conv_IntToString` _battery_power_))
    (else
      (`KismetSystemLibrary.PrintString` (`KismetStringLibrary.Conv_IntToString` _battery_power_))))
  (`self.K2_DestroyActor`))

(fn `UserConstructionScript`)